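; GeniusPawnGestures is a Blueprint that tests touch gesture recognizers by printing debug strings for the gestures it receives.
; Tap, swipe and pan recognizers each drive their own delegate event.
; Tap end prints a double-tap message, and swipe end prints the direction for left, right and up-right diagonal only.
; Pan start prints the first finger's touch X and Y, with no other gameplay effect.
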(event GestureEndedDelegate(TapGestureRecognizer)
  (params (Recognizer :type Gesture%20Recognizer%20Component%20Object%20Reference) (DeltaTime :type Float%20%28single-precision%29))
  ;[1 1 1] Tap Gesture
  (Development|PrintString "Double Tap"))

(event GestureEndedDelegate(SwipeGestureRecognizer)
  (params (Recognizer :type Gesture%20Recognizer%20Component%20Object%20Reference) (DeltaTime :type Float%20%28single-precision%29))
  ;[1 1 1] Swipe Gesture
  (bind _asswipe_gesture_recognizer (Utilities|Casting|CastToSwipeGestureRecognizer Recognizer))
  (bind _returnvalue (Class|SwipeGestureRecognizer|GetSwipeType _asswipe_gesture_recognizer))
  (switch Utilities|FlowControl|Switch|SwitchonESwipeType _returnvalue
    (:SwipeLeft
      (Development|PrintString "Left"))
    (:SwipeRight
      (Development|PrintString "Right"))
    (:SwipeUpRight
      (Development|PrintString "Diagonal Up And Right"))))

(event GestureBeganDelegate(PanGestureRecognizer)
  (params (Recognizer :type Gesture%20Recognizer%20Component%20Object%20Reference) (DeltaTime :type Float%20%28single-precision%29))
  ;[1 1 1] Pan Gesture
  (bind _aspan_gesture_recognizer (Utilities|Casting|CastToPanGestureRecognizer Recognizer))
  (bind _returnvalue (Class|PanGestureRecognizer|FirstFingerTouchLocation _aspan_gesture_recognizer))
  (Development|PrintString (Utilities|String|ToString(Float) (.x _returnvalue)))
  (Development|PrintString (Utilities|String|ToString(Float) (.y _returnvalue))))

(event EventBeginPlay)

(event Collision|EventActorBeginOverlap
  (params (OtherActor :type Actor%20Object%20Reference)))

(event EventTick
  (params (DeltaSeconds :type Float%20%28single-precision%29)))

(fn ConstructionScript)